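; BP_Door is a level door with an entrance and an exit, where an Explorer reaching the exit volume resets the room through BP_GameMode.
; Entrance overlaps trigger timelines that slide the door vertically, opening only if the Explorer's facing passes a dot-product check.
; The exit starts closed and switches collision and material instead of moving.
; Wrapper events expose open and close, though CloseExitEvent actually calls OpenExit.
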(event `PlayAnimationOpenEntrance`
  (bind (_direction _openpercentage) (`Timeline|EntranceDoorOpen` :!via `PlayFromStart`)
    (:`Update`
      (`SceneComponent.K2_SetWorldLocation` (`self.EntranceDoor`) (`KismetMathLibrary.VLerp` (`self.EntranceDoorClosedLocation`) (`self.EntranceDoorOpenLocation`) _openpercentage) false false))))

(event `PlayAnimationCloseEntrance`
  (bind (_direction _openpercentage) (`Timeline|EntranceDoorClose` :!via `PlayFromStart`)
    (:`Update`
      (`SceneComponent.K2_SetWorldLocation` (`self.EntranceDoor`) (`KismetMathLibrary.VLerp` (`self.EntranceDoorClosedLocation`) (`self.EntranceDoorOpenLocation`) _openpercentage) false false))))

(event `self.ReceiveBeginPlay`
  (bind _returnvalue (`SceneComponent.K2_GetComponentLocation` (`self.EntranceDoor`)))
  (`self.CloseExit`)
  (set `self.EntranceDoorOpenLocation` _returnvalue)
  (set `self.EntranceDoorClosedLocation` (- _returnvalue (0.0 0.0 250.0))))

(event `self.Entrance.OnComponentBeginOverlap`
  (params (OverlappedComponent :type "PrimitiveComponent Object Reference") (OtherActor :type "Actor Object Reference") (OtherComp :type "PrimitiveComponent Object Reference") (OtherBodyIndex :type Integer) (bFromSweep :type Boolean) (SweepResult :type "HitResult Structure (by ref)"))
  (bind _asbp_explorer (cast `/Game/OhMummy/Blueprints/Characters/BP_Explorer` OtherActor))
  (if (<= (`KismetMathLibrary.Dot_VectorVector` (`KismetMathLibrary.GetForwardVector` (`self.K2_GetActorRotation` _asbp_explorer)) (`KismetMathLibrary.GetForwardVector` (`self.K2_GetActorRotation`))) 0.0)
    (`self.OpenEntrance`)))

(event `self.Entrance.OnComponentEndOverlap`
  (params (OverlappedComponent :type "PrimitiveComponent Object Reference") (OtherActor :type "Actor Object Reference") (OtherComp :type "PrimitiveComponent Object Reference") (OtherBodyIndex :type Integer))
  (cast `/Game/OhMummy/Blueprints/Characters/BP_Explorer` OtherActor)
  (`self.CloseEntrance`))

(event `self.ExitLevelVolume.OnComponentBeginOverlap`
  (params (OverlappedComponent :type "PrimitiveComponent Object Reference") (OtherActor :type "Actor Object Reference") (OtherComp :type "PrimitiveComponent Object Reference") (OtherBodyIndex :type Integer) (bFromSweep :type Boolean) (SweepResult :type "HitResult Structure (by ref)"))
  (cast `/Game/OhMummy/Blueprints/Characters/BP_Explorer` OtherActor)
  (bind _asbp_game_mode (cast `/Game/OhMummy/Blueprints/Framework/BP_GameMode` (`GameplayStatics.GetGameMode`)))
  (`/Game/OhMummy/Blueprints/Framework/BP_GameMode.ResetRoom` _asbp_game_mode))

(event `self.OpenEntranceEvent`
  (`self.OpenEntrance`))

(event `self.CloseEntranceEvent`
  (`self.CloseEntrance`))

(event `self.OpenExitEvent`
  (`self.OpenExit`))

(event `self.CloseExitEvent`
  (`self.OpenExit`))

(fn `CloseEntrance`
  (bind _entrancedoor (`self.EntranceDoor`))
  (`PrimitiveComponent.SetCollisionResponseToAllChannels` _entrancedoor "ECR_Block")
  (`PrimitiveComponent.SetMaterial` _entrancedoor 0 "/Game/OhMummy/Materials/M_Door_Closed.M_Door_Closed")
  (`self.PlayAnimationCloseEntrance`))

(fn `CloseExit`
  (bind _exitdoor (`self.ExitDoor`))
  (`PrimitiveComponent.SetCollisionResponseToAllChannels` _exitdoor "ECR_Block")
  (`PrimitiveComponent.SetMaterial` _exitdoor 0 "/Game/OhMummy/Materials/M_Door_Closed.M_Door_Closed"))

(fn `OpenEntrance`
  (`PrimitiveComponent.SetMaterial` (`self.EntranceDoor`) 0 "/Game/OhMummy/Materials/M_Door_Closed.M_Door_Closed")
  (`self.PlayAnimationOpenEntrance`))

(fn `OpenExit`
  (bind _exitdoor (`self.ExitDoor`))
  (`PrimitiveComponent.SetCollisionResponseToAllChannels` _exitdoor "ECR_Ignore")
  (`PrimitiveComponent.SetMaterial` _exitdoor 0 "/Game/OhMummy/Materials/M_Door_Open.M_Door_Open"))

(fn `UserConstructionScript`)