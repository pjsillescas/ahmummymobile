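; Oh Mummy sarcophagus block that opens once all four of its edges are activated.
; On BeginPlay it sphere-overlaps for four BP_Junction corners, registers with each and sorts them by quadrant, changing material if the count differs.
; Junction pairs map to edge flags; the full set triggers Open, which reports its content to the GameInstance and spawns extra mummies at a random corner.
; Reset assigns new content and clears the edges.
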(event `self.ReceiveBeginPlay`
  (`self.InitializeSize`)
  (`self.GetVertices`)
  (set `self.NormalMaterial` (`PrimitiveComponent.GetMaterial` (`self.Mesh`) 0)))

(fn `ActivateEdge`
  (params (Vertex1 :type "/Game/OhMummy/Blueprints/Devices/E_Vertices Enum" :default "NewEnumerator0") (Vertex2 :type "/Game/OhMummy/Blueprints/Devices/E_Vertices Enum" :default "NewEnumerator0"))
  (locals (LocalVertex1 :type "/Game/OhMummy/Blueprints/Devices/E_Vertices Enum") (LocalVertex2 :type "/Game/OhMummy/Blueprints/Devices/E_Vertices Enum"))
  (set `local.LocalVertex1` Vertex1)
  (set `local.LocalVertex2` Vertex2)
  (if (`self.IsNorthEdge` (`local.LocalVertex1`) (`local.LocalVertex2`))
    (set `self.bIsNorthEdgeSelected` true)
    (`self.CheckForOpen`)
    (elif (`self.IsSouthEdge` (`local.LocalVertex1`) (`local.LocalVertex2`))
      (set `self.bIsSouthEdgeSelected` true)
      (`self.CheckForOpen`)
      (elif (`self.IsEastEdge` (`local.LocalVertex1`) (`local.LocalVertex2`))
        (set `self.bIsEastEdgeSelected` true)
        (`self.CheckForOpen`)
        (elif (`self.IsWestEdge` (`local.LocalVertex1`) (`local.LocalVertex2`))
          (set `self.bIsWestEdgeSelected` true)
          (`self.CheckForOpen`))))))

(fn `ActivateEdgeVertices`
  (params (Junction1 :type "/Game/OhMummy/Blueprints/Devices/Parts/BP_Junction Object Reference") (Junction2 :type "/Game/OhMummy/Blueprints/Devices/Parts/BP_Junction Object Reference"))
  (`self.ActivateEdge` (`self.GetVertexPosition` Junction1) (`self.GetVertexPosition` Junction2))
  (return))

(fn `ActivateVertex`
  (params (Vertex :type "/Game/OhMummy/Blueprints/Devices/Parts/BP_Junction Object Reference"))
  (locals (LocalVertexPosition :type "/Game/OhMummy/Blueprints/Devices/E_Vertices Enum"))
  (bind _output_get (set `local.LocalVertexPosition` (`self.GetVertexPosition` Vertex)))
  (`self.ActivateEdge` (`self.ActiveVertex`) _output_get))

(fn `CheckForOpen`
  (if (and (`self.bIsNorthEdgeSelected`) (`self.bIsEastEdgeSelected`) (`self.bIsSouthEdgeSelected`) (`self.bIsWestEdgeSelected`))
    (`KismetSystemLibrary.PrintString` (`KismetStringLibrary.Concat_StrStr` (`KismetSystemLibrary.GetDisplayName` self) ": yayyyyyy"))
    (`self.Open`)))

(fn `GetRandomSpawnLocationNearby`
  (returns (Location :type "Vector Structure"))
  (locals (Points :type "Array of Vector Structure"))
  (bind _points (`local.Points`))
  (`|ExecutionSequence`
    (:`then_0`
      (`KismetArrayLibrary.Array_Add` (`local.Points`) (`self.K2_GetActorLocation` (`self.NWVertex`)))
      (`KismetArrayLibrary.Array_Add` (`local.Points`) (`self.K2_GetActorLocation` (`self.NEVertex`)))
      (`KismetArrayLibrary.Array_Add` (`local.Points`) (`self.K2_GetActorLocation` (`self.SWVertex`)))
      (`KismetArrayLibrary.Array_Add` (`local.Points`) (`self.K2_GetActorLocation` (`self.SEVertex`))))
    (:`then_1`
      (return (`|GetArrayItem` _points (`KismetMathLibrary.RandomIntegerInRange` 0 (- (`KismetArrayLibrary.Array_Length` _points) 1)))))))

(fn `GetVertexPosition`
  (params (Vertex :type "/Game/OhMummy/Blueprints/Devices/Parts/BP_Junction Object Reference"))
  (returns (Position :type "/Game/OhMummy/Blueprints/Devices/E_Vertices Enum"))
  (locals (LocalVertex :type "/Game/OhMummy/Blueprints/Devices/E_Vertices Enum"))
  (if (== Vertex (`self.NWVertex`))
    (set `local.LocalVertex` "NewEnumerator1")
    (elif (== Vertex (`self.NEVertex`))
      (set `local.LocalVertex` "NewEnumerator2")
      (elif (== Vertex (`self.SWVertex`))
        (set `local.LocalVertex` "NewEnumerator3")
        (elif (== Vertex (`self.SEVertex`))
          (set `local.LocalVertex` "NewEnumerator4")
          (else
            (set `local.LocalVertex` "NewEnumerator0"))))))
  (return (`local.LocalVertex`)))

(fn `GetVertices`
  (locals (Displacement :type "Vector Structure") (LocalJunction :type "/Game/OhMummy/Blueprints/Devices/Parts/BP_Junction Object Reference"))
  (bind _outactors (`KismetSystemLibrary.SphereOverlapActors` (`self.K2_GetActorLocation`) (* (`KismetMathLibrary.FMax` (`KismetMathLibrary.Conv_IntToDouble` (`self.Width`)) (`KismetMathLibrary.Conv_IntToDouble` (`self.Height`))) 1.2) (`|MakeArray` "ObjectTypeQuery2" :!type "EObjectTypeQuery Enum") "/Game/OhMummy/Blueprints/Devices/Parts/BP_Junction.BP_Junction_C"))
  (if (== (`KismetArrayLibrary.Array_Length` _outactors) 4)
    (for _array_element _outactors
      (bind _asbp_junction (cast `/Game/OhMummy/Blueprints/Devices/Parts/BP_Junction` _array_element))
      (bind _output_get (set `local.LocalJunction` _asbp_junction))
      (`/Game/OhMummy/Blueprints/Devices/Parts/BP_Junction.AddSarcophagus` _output_get self)
      (bind _output_get_2 (set `local.Displacement` (- (`self.K2_GetActorLocation` _output_get) (`self.K2_GetActorLocation`))))
      (bind _returnvalue (>= (.x _output_get_2) 0.0))
      (bind _returnvalue_2 (>= (.y _output_get_2) 0.0))
      (if (and _returnvalue _returnvalue_2)
        (set `self.NEVertex` (`local.LocalJunction`))
        (elif (and (not _returnvalue) _returnvalue_2)
          (set `self.SEVertex` (`local.LocalJunction`))
          (elif (and _returnvalue (not _returnvalue_2))
            (set `self.NWVertex` (`local.LocalJunction`))
            (else
              (set `self.SWVertex` (`local.LocalJunction`)))))))
    (else
      (`PrimitiveComponent.SetMaterial` (`self.Mesh`) 0 "/Engine/MapTemplates/Materials/BasicAsset01.BasicAsset01"))))

(fn `InitializeSize`
  (bind (_origin _boxextent) (`KismetSystemLibrary.GetComponentBounds` (`self.Mesh`)))
  (set `self.Height` (* (`KismetMathLibrary.FTrunc` (.x _boxextent)) 2))
  (set `self.Width` (* (`KismetMathLibrary.FTrunc` (.y _boxextent)) 2)))

(fn `IsEastEdge`
  (params (Vertex1 :type "/Game/OhMummy/Blueprints/Devices/E_Vertices Enum" :default "NewEnumerator0") (Vertex2 :type "/Game/OhMummy/Blueprints/Devices/E_Vertices Enum" :default "NewEnumerator0"))
  (returns (IsNorthEdge :type Boolean))
  (return (or (and (`|EnumEquality` Vertex1 "NewEnumerator2") (`|EnumEquality` Vertex2 "NewEnumerator4")) (and (`|EnumEquality` Vertex1 "NewEnumerator4") (`|EnumEquality` Vertex2 "NewEnumerator2")))))

(fn `IsNorthEdge`
  (params (Vertex1 :type "/Game/OhMummy/Blueprints/Devices/E_Vertices Enum" :default "NewEnumerator0") (Vertex2 :type "/Game/OhMummy/Blueprints/Devices/E_Vertices Enum" :default "NewEnumerator0"))
  (returns (IsNorthEdge :type Boolean))
  (return (or (and (`|EnumEquality` Vertex1 "NewEnumerator1") (`|EnumEquality` Vertex2 "NewEnumerator2")) (and (`|EnumEquality` Vertex1 "NewEnumerator2") (`|EnumEquality` Vertex2 "NewEnumerator1")))))

(fn `IsSouthEdge`
  (params (Vertex1 :type "/Game/OhMummy/Blueprints/Devices/E_Vertices Enum" :default "NewEnumerator0") (Vertex2 :type "/Game/OhMummy/Blueprints/Devices/E_Vertices Enum" :default "NewEnumerator0"))
  (returns (IsNorthEdge :type Boolean))
  (return (or (and (`|EnumEquality` Vertex1 "NewEnumerator3") (`|EnumEquality` Vertex2 "NewEnumerator4")) (and (`|EnumEquality` Vertex1 "NewEnumerator4") (`|EnumEquality` Vertex2 "NewEnumerator3")))))

(fn `IsWestEdge`
  (params (Vertex1 :type "/Game/OhMummy/Blueprints/Devices/E_Vertices Enum" :default "NewEnumerator0") (Vertex2 :type "/Game/OhMummy/Blueprints/Devices/E_Vertices Enum" :default "NewEnumerator0"))
  (returns (IsNorthEdge :type Boolean))
  (return (or (and (`|EnumEquality` Vertex1 "NewEnumerator1") (`|EnumEquality` Vertex2 "NewEnumerator3")) (and (`|EnumEquality` Vertex1 "NewEnumerator3") (`|EnumEquality` Vertex2 "NewEnumerator1")))))

(fn `Open`
  (bind _asbp_game_instance (cast `/Game/OhMummy/Blueprints/Framework/BP_GameInstance` (`GameplayStatics.GetGameInstance`) :!pure true))
  (`PrimitiveComponent.SetMaterial` (`self.Mesh`) 0 "/Engine/MapTemplates/Materials/BasicAsset03.BasicAsset03")
  (switch `/Game/OhMummy/Blueprints/Framework/BP_E_Sarcophagus_Element` (`self.Content`)
    (:`NewEnumerator0`
      (`/Game/OhMummy/Blueprints/Framework/BP_GameInstance.SetKey` _asbp_game_instance))
    (:`NewEnumerator1`
      (`/Game/OhMummy/Blueprints/Framework/BP_GameInstance.SetSarcophagus` _asbp_game_instance))
    (:`NewEnumerator3`
      (`/Game/OhMummy/Blueprints/Framework/BP_GameInstance.AddChest` _asbp_game_instance))
    (:`NewEnumerator4`
      (`/Game/OhMummy/Blueprints/Framework/BP_GameInstance.AddNewMummy` _asbp_game_instance)
      (bind _asbp_game_mode (cast `/Game/OhMummy/Blueprints/Framework/BP_GameMode` (`GameplayStatics.GetGameMode`)))
      (`/Game/OhMummy/Blueprints/Framework/BP_GameMode.SpawnNewMummy` _asbp_game_mode (`self.GetRandomSpawnLocationNearby`)))))

(fn `Reset`
  (params (NewContent :type "/Game/OhMummy/Blueprints/Framework/BP_E_Sarcophagus_Element Enum" :default "NewEnumerator0"))
  (set `self.Content` NewContent)
  (`PrimitiveComponent.SetMaterial` (`self.Mesh`) 0 (`self.NormalMaterial`))
  (set `self.bIsNorthEdgeSelected` false)
  (set `self.bIsEastEdgeSelected` false)
  (set `self.bIsSouthEdgeSelected` false)
  (set `self.bIsWestEdgeSelected` false))

(fn `UserConstructionScript`)