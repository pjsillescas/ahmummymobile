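; Room actor for the Oh Mummy game that procedurally lays out a grid of sarcophagi surrounded by hallways, junctions and border walls.
; BuildRoom runs from both the Construction Script and BeginPlay, placing parts from Rows, Columns, sarcophagus size and hallway width.
; Parts are child actor components offset using the actor's location as relative transform.
; Sarcophagi are stored in an array, and the border pass prints debug row/column indices.
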(event `self.ReceiveBeginPlay`
  (`self.BuildRoom`))

(fn `BuildRoom`
  (locals (LocalRow :type Integer) (LocalColumn :type Integer) (InitialPosition :type "Vector Structure" :default (0.0 0.0 100.0)) (IterationLocationBase :type "Vector Structure"))
  (bind _localrow (`local.LocalRow`))
  (bind _localcolumn (`local.LocalColumn`))
  (set `local.InitialPosition` (`self.K2_GetActorLocation`))
  (for _index (range 1 (+ (`self.Rows`) 1))
    (set `local.LocalRow` _index)
    (for _index_2 (range 1 (+ (`self.Columns`) 1))
      (set `local.LocalColumn` _index_2)
      (bind _spawnedactor (`self.SpawnPartInLocation` (+ (`local.InitialPosition`) (`self.GetSarcophagusLocation` (`local.LocalRow`) (`local.LocalColumn`)) (`KismetMathLibrary.MakeVector` 0.0 0.0 50.0)) (`self.SarcophagusClass`)))
      (`KismetArrayLibrary.Array_Add` (`self.Sarcophaguses`) (cast `/Game/OhMummy/Blueprints/Devices/BP_Sarcophagus` _spawnedactor :!pure true))))
  (for _index_3 (range (+ (`self.Rows`) 1))
    (set `local.LocalRow` _index_3)
    (for _index_4 (range (+ (`self.Columns`) 1))
      (set `local.LocalColumn` _index_4)
      (set `local.IterationLocationBase` (+ (`local.InitialPosition`) (`self.GetSarcophagusLocation` (`local.LocalRow`) (`local.LocalColumn`))))
      (if (or (== _localrow 0) (== _localrow (`self.Rows`)))
        (`self.SpawnPartInLocation` (+ (`local.IterationLocationBase`) (`KismetMathLibrary.MakeVector` (/ (+ (`self.SarcophagusHeight`) (* (`self.HallwayWidth`) -3.0)) 2.0))) (`self.HorizontalWallClass`)))
      (if (or (== _localcolumn 0) (== _localcolumn (`self.Columns`)))
        (`self.SpawnPartInLocation` (+ (`local.IterationLocationBase`) (`KismetMathLibrary.MakeVector` 0.0 (/ (+ (`self.SarcophagusWidth`) (`self.HallwayWidth`)) 2.0) 50.0)) (`self.VerticalWallClass`)))
      (if (> (`local.LocalRow`) 0)
        (`self.SpawnPartInLocation` (+ (`local.IterationLocationBase`) (`KismetMathLibrary.MakeVector` 0.0 (/ (+ (`self.SarcophagusWidth`) (`self.HallwayWidth`)) 2.0))) (`self.VerticalHallwayClass`)))
      (if (> (`local.LocalColumn`) 0)
        (`self.SpawnPartInLocation` (+ (`local.IterationLocationBase`) (`KismetMathLibrary.MakeVector` (/ (+ (`self.SarcophagusHeight`) (`self.HallwayWidth`)) 2.0))) (`self.HorizontalHallwayClass`)))
      (`self.SpawnPartInLocation` (+ (`local.IterationLocationBase`) (`KismetMathLibrary.MakeVector` (/ (+ (`self.SarcophagusHeight`) (`self.HallwayWidth`)) 2.0) (/ (+ (`self.SarcophagusWidth`) (`self.HallwayWidth`)) 2.0))) (`self.JunctionClass`))
      (`KismetSystemLibrary.PrintString` (`KismetStringLibrary.Concat_StrStr` "row: " (`KismetStringLibrary.Conv_IntToString` (`local.LocalRow`)) " col: " (`KismetStringLibrary.Conv_IntToString` (`local.LocalColumn`)))))))

(fn `GetSarcophagusLocation`
  (params (Row :type Integer) (Column :type Integer))
  (returns (Location :type "Vector Structure"))
  (return (`KismetMathLibrary.MakeVector` (+ (* (- Row 1) (`self.SarcophagusHeight`)) (* Row (`self.HallwayWidth`))) (+ (* (- Column 1) (`self.SarcophagusWidth`)) (* Column (`self.HallwayWidth`))) 50.0)))

(fn `SpawnPartInLocation`
  (params (Location :type "Vector Structure") (PartClass :type "Actor Class Reference"))
  (returns (SpawnedActor :type "Actor Object Reference"))
  (bind _returnvalue (`AddComponent|NODE_AddChildActorComponent-4` :`RelativeTransform` (`KismetMathLibrary.MakeTransform` Location)))
  (`ChildActorComponent.SetChildActorClass` _returnvalue PartClass)
  (return (`ChildActorComponent.ChildActor` _returnvalue)))

(fn `UserConstructionScript`
  (`self.BuildRoom`))