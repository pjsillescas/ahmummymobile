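; BP_Junction is a maze junction device in OhMummy that registers the path edges an Explorer travels.
; On collision with an Explorer, it reads that Explorer's last junction, then records itself as the new one.
; If a previous junction exists, it passes that junction and itself as an edge to each sarcophagus in its Sarcophaguses list to activate the matching edge vertices.
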(event `self.OnExplorerCollision`
  (params (Explorer :type "Explorer Object Reference"))
  (bind _returnvalue (`Explorer.GetLastJunction` Explorer))
  (`/Engine/EditorBlueprintResources/StandardMacros.IsValid` Explorer
    (:`Is Valid`
      (`/Engine/EditorBlueprintResources/StandardMacros.IsValid` _returnvalue
        (:`Is Valid`
          (`self.ActivateSarcophagusesWithEdge` _returnvalue))
        (:`Is Not Valid`
          _))
      (`Explorer.SetLastJunction` Explorer self))))

(fn `ActivateSarcophagusesWithEdge`
  (params (Junction :type "Junction Object Reference"))
  (for _array_element (`self.Sarcophaguses`)
    (bind _asbp_sarcophagus (cast `/Game/OhMummy/Blueprints/Devices/BP_Sarcophagus` _array_element))
    (`/Game/OhMummy/Blueprints/Devices/BP_Sarcophagus.ActivateEdgeVertices` _asbp_sarcophagus Junction self))
  (return))

(fn `UserConstructionScript`)