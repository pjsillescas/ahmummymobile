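; Oh Mummy door device with separate entrance and exit doors, each opened or closed by swapping collision response and material.
; An Entrance trigger opens the entrance when a BP_Explorer overlaps while facing against or perpendicular to the door's forward vector, using a dot-product check, and closes it when the overlap ends.
; The exit closes on BeginPlay, and nothing in this Blueprint calls OpenExit.
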(event `self.ReceiveBeginPlay`
  (`self.CloseExit`))

(event `self.Entrance.OnComponentBeginOverlap`
  (params (OverlappedComponent :type "PrimitiveComponent Object Reference") (OtherActor :type "Actor Object Reference") (OtherComp :type "PrimitiveComponent Object Reference") (OtherBodyIndex :type Integer) (bFromSweep :type Boolean) (SweepResult :type "HitResult Structure (by ref)"))
  (bind _asbp_explorer (cast `/Game/OhMummy/Blueprints/Characters/BP_Explorer` OtherActor))
  (if (<= (`KismetMathLibrary.Dot_VectorVector` (`KismetMathLibrary.GetForwardVector` (`self.K2_GetActorRotation` _asbp_explorer)) (`KismetMathLibrary.GetForwardVector` (`self.K2_GetActorRotation`))) 0.0)
    (`self.OpenEntrance`)))

(event `self.Entrance.OnComponentEndOverlap`
  (params (OverlappedComponent :type "PrimitiveComponent Object Reference") (OtherActor :type "Actor Object Reference") (OtherComp :type "PrimitiveComponent Object Reference") (OtherBodyIndex :type Integer))
  (cast `/Game/OhMummy/Blueprints/Characters/BP_Explorer` OtherActor)
  (`self.CloseEntrance`))

(fn `CloseEntrance`
  (bind _entrancedoor (`self.EntranceDoor`))
  (`PrimitiveComponent.SetCollisionResponseToAllChannels` _entrancedoor "ECR_Block")
  (`PrimitiveComponent.SetMaterial` _entrancedoor 0 "/Game/OhMummy/Materials/M_Door_Closed.M_Door_Closed"))

(fn `CloseExit`
  (bind _exitdoor (`self.ExitDoor`))
  (`PrimitiveComponent.SetCollisionResponseToAllChannels` _exitdoor "ECR_Block")
  (`PrimitiveComponent.SetMaterial` _exitdoor 0 "/Game/OhMummy/Materials/M_Door_Closed.M_Door_Closed"))

(fn `OpenEntrance`
  (bind _entrancedoor (`self.EntranceDoor`))
  (`PrimitiveComponent.SetCollisionResponseToAllChannels` _entrancedoor "ECR_Ignore")
  (`PrimitiveComponent.SetMaterial` _entrancedoor 0 "/Game/OhMummy/Materials/M_Door_Open.M_Door_Open"))

(fn `OpenExit`
  (bind _exitdoor (`self.ExitDoor`))
  (`PrimitiveComponent.SetCollisionResponseToAllChannels` _exitdoor "ECR_Ignore")
  (`PrimitiveComponent.SetMaterial` _exitdoor 0 "/Game/OhMummy/Materials/M_Door_Open.M_Door_Open"))

(fn `UserConstructionScript`)