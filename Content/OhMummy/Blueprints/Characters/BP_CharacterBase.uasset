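; Base character for Oh Mummy that handles planar movement relative to control yaw and leaves footprints on the ground.
; Left and right foot triggers trace at their arrow components and spawn footprint decals, stored in an array for bulk clearing.
; A per-tick forward line trace flags obstacles, and capsule overlaps flag Junction occupancy.
; A sphere overlap query reports whether a door is nearby.
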(event `RightFootPrintTrigger`
  (if (`self.bLeaveFootprints`)
    (`self.SetFootprint` (`self.RightFootArrow`))))

(event `LeftFootPrintTrigger`
  (if (`self.bLeaveFootprints`)
    (`self.SetFootprint` (`self.LeftFootArrow`))))

(event `self.ReceiveTick`
  (params (DeltaSeconds :type "Float (single-precision)"))
  (bind _returnvalue (- (`self.K2_GetActorLocation`) (0.0 0.0 25.0)))
  (bind (_outhit _returnvalue_2) (`KismetSystemLibrary.LineTraceSingle` _returnvalue (+ _returnvalue (* (`KismetMathLibrary.GetForwardVector` (`self.K2_GetActorRotation`)) 100.0)) "TraceTypeQuery1"))
  (set `self.bIsAgainstObstacle` _returnvalue_2))

(event `self.CapsuleComponent.OnComponentBeginOverlap`
  (params (OverlappedComponent :type "PrimitiveComponent Object Reference") (OtherActor :type "Actor Object Reference") (OtherComp :type "PrimitiveComponent Object Reference") (OtherBodyIndex :type Integer) (bFromSweep :type Boolean) (SweepResult :type "HitResult Structure (by ref)"))
  (cast `Junction` OtherActor
    (:`then`
      (set `self.bIsInJunction` true))
    (:`CastFailed`
      (set `self.bIsInJunction` false))))

(event `self.CapsuleComponent.OnComponentEndOverlap`
  (params (OverlappedComponent :type "PrimitiveComponent Object Reference") (OtherActor :type "Actor Object Reference") (OtherComp :type "PrimitiveComponent Object Reference") (OtherBodyIndex :type Integer))
  (set `self.bIsInJunction` false))

(fn `ClearFootsteps`
  (for _array_element (`self.Footprints`)
    (`ActorComponent.K2_DestroyComponent` _array_element))
  (`KismetArrayLibrary.Array_Clear` (`self.Footprints`)))

(fn `IsAroundDoor`
  (returns (bIsAroundDoor :type Boolean))
  (bind _outactors (`KismetSystemLibrary.SphereOverlapActors` (`self.K2_GetActorLocation`) 100.0 (`|MakeArray` "ObjectTypeQuery2" :!type "EObjectTypeQuery Enum") "/Game/OhMummy/Blueprints/Devices/BP_Door.BP_Door_C"))
  (return (> (`KismetArrayLibrary.Array_Length` _outactors) 0)))

(fn `MoveForward`
  (params (ScaleValue :type "Float (double-precision)"))
  (`self.AddMovementInput` (`KismetMathLibrary.GetForwardVector` (`KismetMathLibrary.MakeRotator` 0.0 0.0 (.yaw (`self.GetControlRotation`)))) ScaleValue))

(fn `MoveRight`
  (params (ScaleValue :type "Float (double-precision)"))
  (`self.AddMovementInput` (`KismetMathLibrary.GetRightVector` (`KismetMathLibrary.MakeRotator` 0.0 0.0 (.yaw (`self.GetControlRotation`)))) ScaleValue))

(fn `SetFootprint`
  (params (LocationComponent :type "SceneComponent Object Reference"))
  (locals (LocalDisplacement :type "Vector Structure" :default (0.0 0.0 20.0)) (LocalDecalSize :type "Vector Structure" :default (35.0 35.0 35.0)) (LocalDecalSizeF :type "Float (double-precision)" :default 50.0))
  (bind (_returnvalue_roll _returnvalue_pitch _returnvalue_yaw) (`KismetMathLibrary.BreakRotator` (`SceneComponent.K2_GetComponentRotation` LocationComponent)))
  (bind _returnvalue (`SceneComponent.K2_GetComponentLocation` LocationComponent))
  (bind _localdisplacement (`local.LocalDisplacement`))
  (bind _outhit (`KismetSystemLibrary.LineTraceSingle` (- _returnvalue _localdisplacement) (+ _returnvalue _localdisplacement) "TraceTypeQuery1"))
  (bind _returnvalue_2 (`GameplayStatics.SpawnDecalAtLocation` "/Game/OhMummy/Materials/M_footprint.M_footprint" (* (1.0 1.0 1.0) (`local.LocalDecalSizeF`)) (`.Location` (`GameplayStatics.BreakHitResult` _outhit)) (`KismetMathLibrary.MakeRotator` 0.0 90.0 _returnvalue_yaw)))
  (`KismetArrayLibrary.Array_Add` (`self.Footprints`) _returnvalue_2))

(fn `UserConstructionScript`)