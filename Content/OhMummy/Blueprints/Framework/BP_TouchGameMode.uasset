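; Game mode for the touch version of Oh Mummy, running the room cycle, exit door, lives and game over.
; On BeginPlay it caches level actors, adds the HUD and resets the room: shuffled sarcophagus contents, player at start, cleared hallways and footsteps.
; Each reset respawns mummies at shuffled junctions, using the count from the game instance.
; Base-class events trigger room resets, exit opening and life loss, with game over at zero lives.
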(event `SpawnMummies`
  (`self.StopMummies`)
  (bind _asomgame_instance (cast `OMGameInstance` (`GameplayStatics.GetGameInstance`)))
  (`KismetArrayLibrary.Array_Shuffle` (`self.Junctions`))
  (bind (_gamedata_lives _gamedata_score _gamedata_roomnumber _gamedata_bhaskey _gamedata_bhasscroll _gamedata_bhassarcophagus _gamedata_numberofmummies) (break `GameData` (`OMGameInstance.GameData` _asomgame_instance)))
  (for _index (range 1 (+ _gamedata_numberofmummies 1))
    (bind (_returnvalue_x _returnvalue_y) (`KismetMathLibrary.BreakVector` (`self.K2_GetActorLocation` (`|GetArrayItem` (`self.Junctions`) _index))))
    (`self.SpawnNewMummy` (`KismetMathLibrary.MakeVector` _returnvalue_x _returnvalue_y 200.0))))

(event `self.ReceiveBeginPlay`
  (`self.GetReferences`)
  (bind _asbp_touch_player_controller (cast `/Game/OhMummy/Blueprints/Framework/BP_TouchPlayerController` (`GameplayStatics.GetPlayerController` 0)))
  (bind _returnvalue (`|CreateWidget` "/Game/OhMummy/UMG/HUD.HUD_C" null _asbp_touch_player_controller))
  (`UserWidget.AddToViewport` _returnvalue 0)
  (`self.ResetRoom`))

(event `SpawnNewMummy`
  (params (Location :type "Vector Structure"))
  (`|SpawnActorFromClass` "/Game/OhMummy/Blueprints/Characters/BP_Mummy.BP_Mummy_C" (`KismetMathLibrary.MakeTransform` Location) "Undefined" "OverrideRootScale" null null))

(event `OpenExitDoor`
  (`/Game/OhMummy/Blueprints/Devices/BP_Door.OpenExit` (`self.EntranceDoor`)))

(event `AnimatePlayerEnterRoom`
  (bind (_returnvalue_location _returnvalue_rotation) (`KismetMathLibrary.BreakTransform` (`self.GetTransform` (`self.PlayerStart`))))
  (`self.K2_TeleportTo` (`GameplayStatics.GetPlayerPawn` 0) _returnvalue_location _returnvalue_rotation))

(event `GameOver`
  (`self.StopMummies`)
  (`/Game/OhMummy/Blueprints/Framework/BP_TouchPlayerController.DisablePlayerInput` (`self.PlayerController`))
  (bind _returnvalue (`|CreateWidget` "/Game/OhMummy/UMG/GameOverMenu.GameOverMenu_C"))
  (`UserWidget.AddToViewport` _returnvalue 0))

(event `TakeLife`
  (bind _asomgame_instance (cast `OMGameInstance` (`GameplayStatics.GetGameInstance`)))
  (bind _returnvalue (`OMGameInstance.AddLives` _asomgame_instance -1))
  (if (<= _returnvalue 0)
    (`self.GameOver`)))

(event `self.TakeLifeEvent`
  ;[1 1 1] Implementation of OMGameModeBase
  (`self.TakeLife`))

(event `self.ResetRoomEvent`
  ;[1 1 1] Implementation of OMGameModeBase
  (`self.ResetRoom`))

(event `self.OpenExitDoorEvent`
  ;[1 1 1] Implementation of OMGameModeBase
  (`self.OpenExitDoor`))

(fn `GetNearestJunction`
  (returns (NearestJunction :type "/Game/OhMummy/Blueprints/Devices/Parts/BP_Junction Object Reference"))
  (locals (LocalJunction :type "/Game/OhMummy/Blueprints/Devices/Parts/BP_Junction Object Reference") (LocalActorLocation :type "Vector Structure") (MinDistance :type "Float (double-precision)" :default -1.0))
  (set `local.LocalActorLocation` (`self.K2_GetActorLocation` (`GameplayStatics.GetPlayerPawn` 0)))
  (for _array_element (`self.Junctions`)
    (bind _returnvalue (`KismetMathLibrary.Vector_DistanceSquared` (`self.K2_GetActorLocation` _array_element) (`local.LocalActorLocation`)))
    (if (or (< _returnvalue (`local.MinDistance`)) (< (`local.MinDistance`) 0.0))
      (set `local.LocalJunction` _array_element)
      (set `local.MinDistance` _returnvalue)))
  (return (`local.LocalJunction`)))

(fn `GetRandomConfiguration`
  (returns (Configuration :type "Map of Integer to /Game/OhMummy/Blueprints/Framework/BP_E_Sarcophagus_Element Enum"))
  (locals (LocalConfiguration :type "Map of Integer to /Game/OhMummy/Blueprints/Framework/BP_E_Sarcophagus_Element Enum") (Keys :type "Array of Integer"))
  (for _index (range (`KismetArrayLibrary.Array_Length` (`self.Sarcophaguses`)))
    (`KismetArrayLibrary.Array_Add` (`local.Keys`) _index))
  (`KismetArrayLibrary.Array_Shuffle` (`local.Keys`))
  (`|ExecutionSequence`
    (:`then_0`
      (`BlueprintMapLibrary.Map_Add` (`local.LocalConfiguration`) (`|GetArrayItem` (`local.Keys`))))
    (:`then_1`
      (`BlueprintMapLibrary.Map_Add` (`local.LocalConfiguration`) (`|GetArrayItem` (`local.Keys`) 1) "NewEnumerator1"))
    (:`then_2`
      (`BlueprintMapLibrary.Map_Add` (`local.LocalConfiguration`) (`|GetArrayItem` (`local.Keys`) 2) "NewEnumerator5"))
    (:`then_3`
      (`BlueprintMapLibrary.Map_Add` (`local.LocalConfiguration`) (`|GetArrayItem` (`local.Keys`) 3) "NewEnumerator4"))
    (:`then_4`
      (for _index_2 (range 4 11)
        (`BlueprintMapLibrary.Map_Add` (`local.LocalConfiguration`) (`|GetArrayItem` (`local.Keys`) _index_2) "NewEnumerator3"))
      (return (`local.LocalConfiguration`)))))

(fn `GetReferences`
  (bind _outactors (`GameplayStatics.GetAllActorsOfClass` "/Game/OhMummy/Blueprints/Devices/BP_Sarcophagus.BP_Sarcophagus_C"))
  (set `self.Sarcophaguses` _outactors)
  (bind _outactors_2 (`GameplayStatics.GetAllActorsOfClass` "/Script/Engine.PlayerStart"))
  (set `self.PlayerStart` (`|GetArrayItem` _outactors_2))
  (bind _outactors_3 (`GameplayStatics.GetAllActorsOfClass` "/Game/OhMummy/Blueprints/Devices/Parts/BP_Junction.BP_Junction_C"))
  (set `self.Junctions` _outactors_3)
  (bind _outactors_4 (`GameplayStatics.GetAllActorsOfClass` "/Game/OhMummy/Blueprints/Devices/BP_Door.BP_Door_C"))
  (set `self.EntranceDoor` (`|GetArrayItem` _outactors_4))
  (bind _asbp_touch_player_controller (cast `/Game/OhMummy/Blueprints/Framework/BP_TouchPlayerController` (`GameplayStatics.GetPlayerController` 0)))
  (set `self.PlayerController` _asbp_touch_player_controller))

(fn `ResetRoom`
  (locals (Configuration :type "Map of Integer to /Game/OhMummy/Blueprints/Framework/BP_E_Sarcophagus_Element Enum"))
  (`|ExecutionSequence`
    (:`then_0`
      (bind _configuration (`self.GetRandomConfiguration`))
      (set `local.Configuration` _configuration)
      (for (_array_element _array_index) (`self.Sarcophaguses`)
        (bind (_value _returnvalue) (`BlueprintMapLibrary.Map_Find` (`local.Configuration`) _array_index))
        (if _returnvalue
          (`/Game/OhMummy/Blueprints/Devices/BP_Sarcophagus.Reset` _array_element _value)
          (else
            (`/Game/OhMummy/Blueprints/Devices/BP_Sarcophagus.Reset` _array_element "NewEnumerator2")))))
    (:`then_1`
      (`self.AnimatePlayerEnterRoom`))
    (:`then_2`
      (`/Game/OhMummy/Blueprints/Devices/BP_Door.CloseExit` (`self.EntranceDoor`))
      (`/Game/OhMummy/Blueprints/Devices/BP_Door.OpenEntrance` (`self.EntranceDoor`)))
    (:`then_3`
      (bind _asomgame_instance (cast `OMGameInstance` (`GameplayStatics.GetGameInstance`)))
      (`OMGameInstance.EnterRoom` _asomgame_instance))
    (:`then_4`
      (bind _outactors (`GameplayStatics.GetAllActorsOfClass` "/Game/OhMummy/Blueprints/Devices/Parts/BP_HorizontalHallway.BP_HorizontalHallway_C"))
      (`/Game/OhMummy/Blueprints/Devices/Parts/BP_HorizontalHallway.SetTraversed` _outactors false)
      (bind _outactors_2 (`GameplayStatics.GetAllActorsOfClass` "/Game/OhMummy/Blueprints/Devices/Parts/BP_VerticalHallway.BP_VerticalHallway_C"))
      (`/Game/OhMummy/Blueprints/Devices/Parts/BP_VerticalHallway.SetTraversed` _outactors_2 false)
      (bind _asbp_character_base (cast `/Game/OhMummy/Blueprints/Characters/BP_CharacterBase` (`GameplayStatics.GetPlayerPawn` 0)))
      (`/Game/OhMummy/Blueprints/Characters/BP_CharacterBase.ClearFootsteps` _asbp_character_base))
    (:`then_5`
      (`self.SpawnMummies`)
      (`/Game/OhMummy/Blueprints/Framework/BP_TouchPlayerController.EnablePlayerInput` (`self.PlayerController`)))
    (:`then_6`
      (`self.StartBackgroundMusic`))))

(fn `StartBackgroundMusic`
  (if (not (`self.bIsSoundPlaying`))
    (`GameplayStatics.PlaySoundAtLocation` "/Game/OhMummy/Sounds/Background_Music_Cue.Background_Music_Cue" (`self.K2_GetActorLocation` (`GameplayStatics.GetPlayerCameraManager` 0)) (struct) 1.0 1.0 0.0 null null null)
    (set `self.bIsSoundPlaying` true)))

(fn `StopMummies`
  (bind _outactors (`GameplayStatics.GetAllActorsOfClass` "/Game/OhMummy/Blueprints/Characters/BP_Mummy.BP_Mummy_C"))
  (for _array_element _outactors
    (`self.K2_DestroyActor` _array_element))
  (return))

(fn `UserConstructionScript`)