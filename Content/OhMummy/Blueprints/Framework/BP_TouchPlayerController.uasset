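; Player controller for Oh Mummy that steers the character in four directions from touch swipes or movement axis inputs.
; A swipe past a distance threshold fires once per touch and picks its direction from the dominant axis.
; Tick keeps the character moving, buffering each new direction until a junction, obstacle, door or reversal allows the turn.
; BeginPlay blends to the level camera before enabling movement, and helper functions toggle between game and UI input.
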(event `self.ReceiveBeginPlay`
  (bind _asbp_character_base (cast `/Game/OhMummy/Blueprints/Characters/BP_CharacterBase` (`GameplayStatics.GetPlayerPawn` 0)))
  (set `self.PlayerCharacter` _asbp_character_base)
  (bind _outactors (`GameplayStatics.GetAllActorsOfClass` "/Script/Engine.PlayerStart"))
  (set `self.PlayerStart` (`|GetArrayItem` _outactors))
  (set `self.bCanMove` false)
  (`self.AnimateCameraToInitialPosition`)
  (`KismetSystemLibrary.Delay` (`self.CameraTravelingTime`))
  (set `self.bCanMove` true))

(event `self.ReceiveTick`
  (params (DeltaSeconds :type "Float (single-precision)"))
  (bind (_locationx _locationy) (`self.GetInputTouchState` "Touch1"))
  (`self.ProcessMovement`)
  (if (`self.bIsPressed`)
    (if (> (`KismetMathLibrary.VSize2D` (- (`self.TouchStart`) (`KismetMathLibrary.MakeVector2D` _locationx _locationy))) (`self.SwipeDistance`))
      (`/Engine/EditorBlueprintResources/StandardMacros.DoOnce` false :!label _label
        (:`Completed`
          (`self.ProcessSwipe`))))))

(event `InputTouch`
  (params (Location :type "Vector Structure") (FingerIndex :type "ETouchIndex Enum"))
  (bind (_locationx _locationy) (`self.GetInputTouchState` "Touch1"))
  (:`Pressed`
    (set `self.bIsPressed` true)
    (set `self.TouchStart` (`KismetMathLibrary.MakeVector2D` _locationx _locationy)))
  (:`Released`
    (set `self.bIsPressed` false)
    (goto _label :!via `Reset`)))

(event `ProcessSwipe`
  (bind (_locationx _locationy) (`self.GetInputTouchState` "Touch1"))
  (bind (_x _y) (`KismetMathLibrary.BreakVector2D` (- (`self.TouchStart`) (`self.TouchEnd`))))
  (set `self.TouchEnd` (`KismetMathLibrary.MakeVector2D` _locationx _locationy))
  (if (> (`KismetMathLibrary.Abs` _x) (`KismetMathLibrary.Abs` _y))
    (if (> _x 0.0)
      (`KismetSystemLibrary.PrintString` "Left")
      (`self.MoveRight` -1.0)
      (else
        (`KismetSystemLibrary.PrintString` "Right")
        (`self.MoveRight` 1.0)))
    (elif (> _y 0.0)
      (`KismetSystemLibrary.PrintString` "Up")
      (`self.MoveForward` 1.0)
      (else
        (`KismetSystemLibrary.PrintString` "Down")
        (`self.MoveForward` -1.0)))))

(event `ProcessMovement`
  (bind _playercharacter (`self.PlayerCharacter`))
  (if (`|EnumInequality` (`self.DesiredMovement`) "NewEnumerator4")
    (if (or (`/Game/OhMummy/Blueprints/Characters/BP_CharacterBase.bIsInJunction` _playercharacter) (`/Game/OhMummy/Blueprints/Characters/BP_CharacterBase.bIsAgainstObstacle` _playercharacter) (`self.AreOppositeMovements` (`self.CurrentMovement`) (`self.DesiredMovement`)) (`/Game/OhMummy/Blueprints/Characters/BP_CharacterBase.IsAroundDoor` (`self.PlayerCharacter`)))
      (set `self.CurrentMovement` (`self.DesiredMovement`))
      (set `self.DesiredMovement` "NewEnumerator4")))
  (switch `/Game/OhMummy/Blueprints/Framework/BP_E_MovementDirection` (`self.CurrentMovement`)
    (:`NewEnumerator0`
      (`/Game/OhMummy/Blueprints/Characters/BP_CharacterBase.MoveRight` (`self.PlayerCharacter`) -1.0))
    (:`NewEnumerator1`
      (`/Game/OhMummy/Blueprints/Characters/BP_CharacterBase.MoveRight` (`self.PlayerCharacter`) 1.0))
    (:`NewEnumerator2`
      (`/Game/OhMummy/Blueprints/Characters/BP_CharacterBase.MoveForward` (`self.PlayerCharacter`) 1.0))
    (:`NewEnumerator3`
      (`/Game/OhMummy/Blueprints/Characters/BP_CharacterBase.MoveForward` (`self.PlayerCharacter`) -1.0))))

(event `InputAxis|MoveForward`
  (params (AxisValue :type "Float (single-precision)"))
  ;[1 1 1] Controller Moves
  (`self.MoveForward` AxisValue))

(event `InputAxis|MoveRight`
  (params (AxisValue :type "Float (single-precision)"))
  ;[1 1 1] Controller Moves
  (`self.MoveRight` AxisValue))

(fn `AnimateCameraToInitialPosition`
  (bind _outactors (`GameplayStatics.GetAllActorsOfClass` "/Script/Engine.CameraActor"))
  (`self.SetViewTargetWithBlend` (`|GetArrayItem` _outactors) (`self.CameraTravelingTime`))
  (return))

(fn `AreMovementPair`
  (params (Movement1 :type "/Game/OhMummy/Blueprints/Framework/BP_E_MovementDirection Enum" :default "NewEnumerator0") (Movement2 :type "/Game/OhMummy/Blueprints/Framework/BP_E_MovementDirection Enum" :default "NewEnumerator0") (Value1 :type "/Game/OhMummy/Blueprints/Framework/BP_E_MovementDirection Enum" :default "NewEnumerator0") (Value2 :type "/Game/OhMummy/Blueprints/Framework/BP_E_MovementDirection Enum" :default "NewEnumerator0"))
  (returns (bArePair :type Boolean))
  (return (or (and (`|EnumEquality` Movement1 Value1) (`|EnumEquality` Movement2 Value2)) (and (`|EnumEquality` Movement1 Value2) (`|EnumEquality` Movement2 Value1)))))

(fn `AreOppositeMovements`
  (params (Movement1 :type "/Game/OhMummy/Blueprints/Framework/BP_E_MovementDirection Enum" :default "NewEnumerator0") (Movement2 :type "/Game/OhMummy/Blueprints/Framework/BP_E_MovementDirection Enum" :default "NewEnumerator0"))
  (returns (AreOpposite :type Boolean))
  (return (or (`self.AreMovementPair` Movement1 Movement2 "NewEnumerator0" "NewEnumerator1") (`self.AreMovementPair` Movement1 Movement2 "NewEnumerator2" "NewEnumerator3"))))

(fn `ChangeMovement`
  (params (NewMovement :type "/Game/OhMummy/Blueprints/Framework/BP_E_MovementDirection Enum" :default "NewEnumerator0"))
  (if (`|EnumEquality` (`self.CurrentMovement`) "NewEnumerator4")
    (set `self.CurrentMovement` NewMovement)
    (else
      (set `self.DesiredMovement` NewMovement))))

(fn `DisablePlayerInput`
  (`WidgetBlueprintLibrary.SetInputMode_UIOnlyEx` self null)
  (`self.DisableInput` (`self.K2_GetPawn`) self)
  (set `self.bShowMouseCursor` true)
  (set `self.bCanMove` false)
  (return))

(fn `EnablePlayerInput`
  (`WidgetBlueprintLibrary.SetInputMode_GameOnly` self)
  (`self.EnableInput` (`self.K2_GetPawn`) self)
  (set `self.bShowMouseCursor` false)
  (set `self.bCanMove` true)
  (return))

(fn `MoveForward`
  (params (ScaleValue :type "Float (double-precision)"))
  (if (`self.bCanMove`)
    (if (> ScaleValue 0.0)
      (`self.ChangeMovement` "NewEnumerator2")
      (elif (< ScaleValue 0.0)
        (`self.ChangeMovement` "NewEnumerator3")))))

(fn `MoveRight`
  (params (ScaleValue :type "Float (double-precision)"))
  (if (`self.bCanMove`)
    (if (> ScaleValue 0.0)
      (`self.ChangeMovement` "NewEnumerator1")
      (elif (< ScaleValue 0.0)
        (`self.ChangeMovement` "NewEnumerator0")))))

(fn `UserConstructionScript`)