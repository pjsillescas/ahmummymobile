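; Game instance for Oh Mummy that manages the persistent top-score table.
; It loads the table from a BP_TopScores save slot, or creates that save from its in-memory list when none exists.
; CheckForTopScore finds the first entry the current GameData score meets or beats.
; UpdateTopScoreList inserts the named, dated score at a given index and drops the last entry, while OverwriteTopScoresSave separately writes the list to disk.
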(fn `CheckForTopScore`
  (returns (IsTopNewScore :type Boolean) (TopScoreIndex :type Integer))
  (locals (LocalTopNewScore :type Boolean) (LocalIndex :type Integer))
  (bind (_gamedata_lives _gamedata_score) (break `GameData` (`self.GameData`)))
  (for (_array_element _array_index) (`self.TopScoresInst`)
    (set `local.LocalIndex` _array_index)
    (if (>= _gamedata_score (`.PlayerScore_5_BDDCCBB8405A03B8F7B35EAAC6DA5AE2` (break `/Game/OhMummy/UMG/S_TopScores` _array_element)))
      (set `local.LocalTopNewScore` true)
      (break)))
  (return (`local.LocalTopNewScore`) (`local.LocalIndex`)))

(fn `CreateTopScoresSave`
  (bind _returnvalue (`GameplayStatics.CreateSaveGameObject` "/Game/OhMummy/UMG/BP_TopScores.BP_TopScores_C"))
  (bind _output_get (set `self.TopScoresObj` _returnvalue))
  (set `/Game/OhMummy/UMG/BP_TopScores.TopScores` (`self.TopScoresInst`) _output_get)
  (`GameplayStatics.SaveGameToSlot` (`self.TopScoresObj`) (`self.TopScoresSlot`))
  (`KismetSystemLibrary.PrintString` "Brand new scores created!!"))

(fn `GetTopScoresList`
  (returns (TopScoresInst :type "Array of /Game/OhMummy/UMG/S_TopScores Structure"))
  (bind _returnvalue (`GameplayStatics.DoesSaveGameExist` (`self.TopScoresSlot`)))
  (if _returnvalue
    (`self.LoadTopScoresSave`)
    (else
      (`self.CreateTopScoresSave`)))
  (return (`self.TopScoresInst`)))

(fn `LoadTopScoresSave`
  (bind _returnvalue (`GameplayStatics.DoesSaveGameExist` (`self.TopScoresSlot`)))
  (if _returnvalue
    (bind _returnvalue_2 (`GameplayStatics.LoadGameFromSlot` (`self.TopScoresSlot`)))
    (bind _asbp_top_scores (cast `/Game/OhMummy/UMG/BP_TopScores` _returnvalue_2))
    (bind _output_get (set `self.TopScoresObj` _asbp_top_scores))
    (set `self.TopScoresInst` (`/Game/OhMummy/UMG/BP_TopScores.TopScores` _output_get))
    (`KismetSystemLibrary.PrintString` "Loaded top scores!!")
    (else
      (`KismetSystemLibrary.PrintString` "No top scores save exist!!!"))))

(fn `OverwriteTopScoresSave`
  (bind _topscoresobj (`self.TopScoresObj`))
  (`/Engine/EditorBlueprintResources/StandardMacros.IsValid` _topscoresobj
    (:`Is Valid`
      (set `/Game/OhMummy/UMG/BP_TopScores.TopScores` (`self.TopScoresInst`) _topscoresobj)
      (`GameplayStatics.SaveGameToSlot` (`self.TopScoresObj`) (`self.TopScoresSlot`))
      (`KismetSystemLibrary.PrintString` "Overwrite Top score!!"))
    (:`Is Not Valid`
      (`self.CreateTopScoresSave`))))

(fn `UpdateTopScoreList`
  (params (PlayerName :type Text) (SlotToScoreIn :type Integer))
  (bind _topscoresinst (`self.TopScoresInst`))
  (bind (_gamedata_lives _gamedata_score) (break `GameData` (`self.GameData`)))
  (`KismetArrayLibrary.Array_Insert` (`self.TopScoresInst`) (make `/Game/OhMummy/UMG/S_TopScores` PlayerName _gamedata_score (`KismetMathLibrary.Today`)) SlotToScoreIn)
  (`KismetArrayLibrary.Array_Remove` _topscoresinst (`KismetArrayLibrary.Array_LastIndex` _topscoresinst))
  (return))