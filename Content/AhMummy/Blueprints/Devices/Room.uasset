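; Room actor that procedurally lays out an Ah Mummy level as a Rows by Columns grid of sarcophagi.
; BuildRoom spawns and records the sarcophagi, then adds hallways, junctions and walls along the first and last rows.
; Positions are offsets from the actor using hard-coded cell and corridor sizes, partly through GetSarcophagusLocation.
; BuildRoom runs from both the construction script and BeginPlay, with no cleanup of earlier spawns.
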(event `self.ReceiveBeginPlay`
  (`self.BuildRoom`))

(fn `BuildRoom`
  (locals (LocalRow :type Integer) (LocalColumn :type Integer) (InitialPosition :type "Vector Structure" :default (0.0 0.0 100.0)))
  (bind _localcolumn (`local.LocalColumn`))
  (bind _localrow (`local.LocalRow`))
  (bind _localcolumn_2 (`local.LocalColumn`))
  (bind _localrow_2 (`local.LocalRow`))
  (bind _localcolumn_3 (`local.LocalColumn`))
  (bind _localrow_3 (`local.LocalRow`))
  (bind _localcolumn_4 (`local.LocalColumn`))
  (bind _localrow_4 (`local.LocalRow`))
  (bind _localcolumn_5 (`local.LocalColumn`))
  (bind _localrow_5 (`local.LocalRow`))
  (bind _localcolumn_6 (`local.LocalColumn`))
  (bind _localrow_6 (`local.LocalRow`))
  (set `local.InitialPosition` (`self.K2_GetActorLocation`))
  (for _index (range 1 (+ (`self.Rows`) 1))
    (set `local.LocalRow` _index)
    (for _index_2 (range 1 (+ (`self.Columns`) 1))
      (set `local.LocalColumn` _index_2)
      (bind _returnvalue (`|SpawnActorFromClass` "/Game/AhMummy/Blueprints/Devices/BP_Sarcophagus.BP_Sarcophagus_C" (`KismetMathLibrary.MakeTransform` (+ (`local.InitialPosition`) (`KismetMathLibrary.MakeVector` (+ (* (- _localrow_6 1) 312.0) (* _localrow_6 85.0)) (+ (* (- _localcolumn 1) 504.0) (* _localcolumn 85.0)) 100.0))) "Undefined" "OverrideRootScale" null null))
      (`KismetArrayLibrary.Array_Add` (`self.Sarcophaguses`) _returnvalue)))
  (for _index_3 (range (+ (`self.Rows`) 1))
    (set `local.LocalRow` _index_3)
    (for _index_4 (range (+ (`self.Columns`) 1))
      (set `local.LocalColumn` _index_4)
      (if (or (== _localrow_4 0) (== _localrow_4 (`self.Rows`)))
        (`|SpawnActorFromClass` "/Game/AhMummy/Blueprints/Devices/Parts/BP_HorizontalWall.BP_HorizontalWall_C" (`KismetMathLibrary.MakeTransform` (+ (`local.InitialPosition`) (`self.GetSarcophagusLocation` (`local.LocalRow`) (`local.LocalColumn`)) (`KismetMathLibrary.MakeVector` (/ (+ 312.0 (* 86.0 -3.0)) 2.0)))) "Undefined" "OverrideRootScale" null null)
        (if (or (== _localcolumn_5 0) (== _localcolumn_5 (`self.Columns`)))
          (`|SpawnActorFromClass` "/Game/AhMummy/Blueprints/Devices/Parts/BP_VerticalHallway.BP_VerticalHallway_C" (`KismetMathLibrary.MakeTransform` (+ (`local.InitialPosition`) (`KismetMathLibrary.MakeVector` (+ (* (- _localrow_2 1) 312.0) (* _localrow_2 85.0) 0.0) (+ (* (- _localcolumn_3 1) 504.0) (* _localcolumn_3 85.0) (/ (+ 504.0 86.0) 2.0)) 50.0))) "Undefined" "OverrideRootScale" null null)))
      (if (> (`local.LocalRow`) 0)
        (`|SpawnActorFromClass` "/Game/AhMummy/Blueprints/Devices/Parts/BP_VerticalHallway.BP_VerticalHallway_C" (`KismetMathLibrary.MakeTransform` (+ (`local.InitialPosition`) (`KismetMathLibrary.MakeVector` (+ (* (- _localrow_3 1) 312.0) (* _localrow_3 85.0) 0.0) (+ (* (- _localcolumn_4 1) 504.0) (* _localcolumn_4 85.0) (/ (+ 504.0 86.0) 2.0)) 50.0))) "Undefined" "OverrideRootScale" null null))
      (if (> (`local.LocalColumn`) 0)
        (`|SpawnActorFromClass` "/Game/AhMummy/Blueprints/Devices/Parts/BP_HorizontalHallway.BP_HorizontalHallway_C" (`KismetMathLibrary.MakeTransform` (+ (`local.InitialPosition`) (`KismetMathLibrary.MakeVector` (+ (* (- _localrow_5 1) 312.0) (* _localrow_5 85.0) (/ (+ 312.0 86.0) 2.0)) (+ (* (- _localcolumn_6 1) 504.0) (* _localcolumn_6 85.0) 0.0) 50.0))) "Undefined" "OverrideRootScale" null null))
      (`|SpawnActorFromClass` "/Game/AhMummy/Blueprints/Devices/Parts/BP_Junction.BP_Junction_C" (`KismetMathLibrary.MakeTransform` (+ (`local.InitialPosition`) (`KismetMathLibrary.MakeVector` (+ (* (- _localrow 1) 312.0) (* _localrow 85.0) (/ (+ 312.0 86.0) 2.0)) (+ (* (- _localcolumn_2 1) 504.0) (* _localcolumn_2 85.0) (/ (+ 504.0 86.0) 2.0)) 50.0))) "Undefined" "OverrideRootScale" null null))))

(fn `GetSarcophagusLocation`
  (params (Row :type Integer) (Column :type Integer))
  (returns (Location :type "Vector Structure"))
  (return (`KismetMathLibrary.MakeVector` (+ (* (- Row 1) 312.0) (* Row 85.0)) (+ (* (- Column 1) 504.0) (* Column 85.0)) 50.0)))

(fn `UserConstructionScript`
  (`self.BuildRoom`))